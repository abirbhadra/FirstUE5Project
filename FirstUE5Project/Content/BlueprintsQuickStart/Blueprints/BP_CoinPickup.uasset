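; Coin pickup that hides itself, disables collision and plays a sound when any actor overlaps it, then respawns on a timer.
; PickedUp and the respawn event share a visibility and collision toggle.
; Respawn plays a double-speed timeline that drives the coin mesh's height and adds roll spin.
; The construction script scales the mesh by NumberOfCoinsToGive, though no coins are awarded in this Blueprint.
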(event `self.ReceiveBeginPlay`)

(event `self.ReceiveTick`
  (params (DeltaSeconds :type "Float (single-precision)")))

(event `self.ReceiveActorBeginOverlap`
  (params (OtherActor :type "Actor Object Reference"))
  (`self.PickedUp`)
  (bind _returnvalue (`KismetSystemLibrary.K2_SetTimerDelegate` (`|CreateDelegate` :!event `RespawnPickup`) (`self.TimeBeforeRespawing`)))
  (set `self.RespawnTimer` _returnvalue))

(event `PlayPickupSound`
  ;[1 1 1] PlaySound
  (`GameplayStatics.PlaySoundAtLocation` "/Game/StarterContent/Audio/Explosion_Cue.Explosion_Cue" (`self.K2_GetActorLocation`) (struct) 1.0 1.0 0.0 null null null null))

(event `RespawnPickup`
  (bind _sm_coin (`self.SM_Coin`))
  (`self.ToggleVisiblityandCollision` false)
  (`TimelineComponent.SetPlayRate` (`self.T_RespawnAnimation`) 2.0)
  (bind (_direction _zmovement _newrollrotation) (`Timeline|T_RespawnAnimation` :!via `PlayFromStart`)
    (:`Update`
      (`SceneComponent.K2_SetRelativeLocation` _sm_coin (`KismetMathLibrary.MakeVector` 0.0 0.0 _zmovement) false false)
      (`SceneComponent.K2_AddRelativeRotation` _sm_coin (`KismetMathLibrary.MakeRotator` _newrollrotation) false false))))

(fn `PickedUp`
  (`self.ToggleVisiblityandCollision` true)
  (`self.PlayPickupSound`))

(fn `ToggleVisiblityandCollision`
  (params (ShouldHide :type Boolean))
  (`self.SetActorHiddenInGame` (select `bool` ShouldHide :`true` true))
  (`|ExecutionSequence`
    (:`then_0`
      (`SceneComponent.SetVisibility` (`self.SM_Coin`) true false))
    (:`then_1`
      (`self.SetActorEnableCollision` (select `bool` ShouldHide :`false` true)))))

(fn `UserConstructionScript`
  (`SceneComponent.SetRelativeScale3D` (`self.SM_Coin`) (select `int` (`self.NumberOfCoinsToGive`) :`0` (1.0 1.0 0.25) :`1` (1.0 1.0 0.25) :`2` (2.0 2.0 0.25) :!type "Vector Structure")))